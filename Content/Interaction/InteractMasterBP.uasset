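; InteractMasterBP is a master interactable actor that reacts to being looked at, hovered and interacted with, using debug prints as default responses.
; Look events accumulate current and total gaze time in a 2D vector, resetting the current value when looking ends.
; Hover sets reach and toggles custom depth on the object when PublicInteraction is enabled.
; Interaction branches on reach into separate action events, printing look stats when in reach, and counts completed interactions.
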(event Custom|StartInteract
  ;[1 1 1] InteractionLogic
  (if (Variables|Default|GetInReach?)
    (CallFunction|InReachInteractAction)
    (else
      (CallFunction|OutReachInteractAction))))

(event Custom|OutReachInteractAction
  ;[1 1 1] Interaction Actions
  (Development|PrintString "Look at me!"))

(event Custom|EndInteractAction
  ;[1 1 1] Interaction Actions
  (Development|PrintString "End Interact"))

(event Custom|StartLook
  ;[1 1 1] Looking
  (Variables|Stats|SetLookTime (+ (Variables|Stats|GetLookTime) (Variables|Default|GetTick)))
  (if (not (Variables|Default|GetLookedAt?))
    (Variables|Default|SetLookedAt? true)
    (Development|PrintString "Hi!")))

(event Custom|EndHover
  ;[1 1 1] HoverLogic
  (Variables|Default|SetInReach? false)
  (if (Variables|Default|GetPublicInteraction?)
    (Rendering|SetRenderCustomDepth (Variables|Default|GetObject) false)))

(event Custom|EndInteract
  ;[1 1 1] InteractionLogic
  (CallFunction|EndInteractAction)
  (Math|Integer|IncrementInt (Variables|Stats|GetInteractCount)))

(event Custom|StartHover
  ;[1 1 1] HoverLogic
  (Variables|Default|SetInReach? true)
  (if (Variables|Default|GetPublicInteraction?)
    (Rendering|SetRenderCustomDepth (Variables|Default|GetObject) true)))

(event Custom|EndLook
  ;[1 1 1] End Looking
  (if (Variables|Default|GetLookedAt?)
    (Variables|Default|SetLookedAt? false)
    (Development|PrintString "Bye then!")
    (Variables|Stats|SetLookTime (Math|Vector2D|MakeVector2D 0.0 (.y (Variables|Stats|GetLookTime))))
    (CallFunction|EndHover)))

(event Custom|InReachInteractAction
  ;[1 1 1] Interaction Actions
  (Stats|DisplayLookStats))

(event EventBeginPlay)

(event Collision|EventActorBeginOverlap
  (params (OtherActor :type Actor%20Object%20Reference)))

(event EventTick
  (params (DeltaSeconds :type Float%20%28single-precision%29))
  (Variables|Default|SetTick DeltaSeconds))

(fn ConstructionScript)

(fn DisplayLookStats
  (bind _looktime (Variables|Stats|GetLookTime))
  (Development|PrintString (Utilities|String|Append "You've looked at this for " (Utilities|String|ToString(Integer) (Math|Float|Round (.x _looktime))) " seconds (" (Utilities|String|ToString(Integer) (Math|Float|Round (.y _looktime))) " seconds in total)")))