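; Master pickup actor that the player can grab and carry as a physics object through interact events inherited or received from the interaction system.
; On interact it adds a temporary physics handle to the player character, grabs its Object component and ignores Pawn collision.
; Tick moves the handle to a raised point ahead of the player, following control rotation.
; Ending interaction releases and destroys the handle and restores Pawn blocking.
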(event EventBeginPlay
  (|CallParentFunction) ; This node is disabled and will not be called.\nDrag off pins to build functionality.
)

(event Collision|EventActorBeginOverlap
  (params (OtherActor :type Actor%20Object%20Reference))
  (|CallParentFunction OtherActor) ; This node is disabled and will not be called.\nDrag off pins to build functionality.
)

(event EventTick
  (params (DeltaSeconds :type Float%20%28single-precision%29))
  (bind _returnvalue (Game|GetPlayerCharacter 0))
  (bind _returnvalue_2 (Pawn|GetControlRotation _returnvalue :!class /Script/Engine.Pawn))
  (|CallParentFunction DeltaSeconds)
  (if (Variables|Default|GetPhysicsHandleActive)
    (Variables|Default|SetHandleLocation (+ (+ (Transformation|GetActorLocation _returnvalue) (* (Math|Vector|GetForwardVector _returnvalue_2) (Variables|Default|GetHoldDistance))) "0, 0,50.000000"))
    (Class|PhysicsHandleComponent|SetTargetLocationandRotation (Variables|Default|GetPhysicsHandle) (Variables|Default|GetHandleLocation) _returnvalue_2)))

(event EventInReachInteractAction
  (Variables|Default|SetPhysicsHandleActive true)
  (bind _returnvalue (AddComponent|AddPhysicsHandleComponent (Game|GetPlayerCharacter 0)))
  (bind _output_get (Variables|Default|SetPhysicsHandle _returnvalue))
  (Physics|Components|PhysicsHandle|GrabComponentatLocationwithRotation _output_get (Variables|Default|GetObject) "None" (Transformation|GetActorLocation) "0, 0, 0")
  (Collision|SetCollisionResponsetoChannel (Variables|Default|GetObject) "ECC_Pawn" "ECR_Ignore"))

(event EventEndInteractAction
  (bind _physicshandle (Variables|Default|GetPhysicsHandle))
  (if (Variables|Default|GetPhysicsHandleActive)
    (Variables|Default|SetPhysicsHandleActive false)
    (Physics|Components|PhysicsHandle|ReleaseComponent _physicshandle)
    (Components|DestroyComponent _physicshandle)
    (Collision|SetCollisionResponsetoChannel (Variables|Default|GetObject) "ECC_Pawn" "ECR_Block")))

(fn ConstructionScript
  (|CallParentFunction))